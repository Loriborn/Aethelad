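; AI controller for an RTS unit character that chases the player pawn shortly after spawning and makes one attack attempt when the move finishes.
; Incoming hits map attack direction to slash, pierce or bludgeon, then apply that type's threshold and resistance to health.
; Damaging hits launch the unit and spawn blood, while ineffective ones stun an attacking player hero.
; Death removes the unit from the shared renderer and destroys pawn and controller.
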(event `TryToAttack`
  (bind _asaethelad_player_character_base (cast `/Game/RTS/Blueprints/Player/AetheladPlayerCharacter/AetheladPlayerCharacterBase` (`self.K2_GetPawn` (`GameplayStatics.GetPlayerControllerFromID` 0)) :!pure true))
  (`/Engine/EditorBlueprintResources/StandardMacros.IsValid` _asaethelad_player_character_base
    (:`Is Valid`
      (`/Game/RTS/Blueprints/Player/AetheladPlayerCharacter/AetheladPlayerCharacterBase.ReceiveDamage` _asaethelad_player_character_base false "NewEnumerator1" 5 (0.0 0.0 300.0) self))))

(event `self.ReceiveBeginPlay`
  (`KismetSystemLibrary.Delay` 1.0)
  (`AITask_MoveTo.AIMoveTo` self (0.0 0.0 0.0) (`self.K2_GetPawn` (`GameplayStatics.GetPlayerControllerFromID` 0)) 10.0
    (:`OnMoveFinished`
      (`self.TryToAttack`))))

(event `CharacterDie`
  (`KismetSystemLibrary.PrintString` "ugh i am slain")
  (`GameplayStatics.PlaySoundAtLocation` "/Game/RTS/Assets/Sounds/Attack/Attack_Death.Attack_Death" (`self.K2_GetActorLocation`) (struct) 1.0 1.0 0.0 null null null)
  (`/Game/RTS/Blueprints/AI/AICharacterRenderer.RemoveUnit` (`/Game/RTS/Blueprints/Game/AetheladGameInstance.AIUnitCharacterRenderer` (cast `/Game/RTS/Blueprints/Game/AetheladGameInstance` (`GameplayStatics.GetGameInstance`) :!pure true)) (`self.Index`))
  (`self.K2_DestroyActor` (`self.K2_GetPawn`))
  (`self.K2_DestroyActor`))

(event `ReceiveDamage`
  (params (ReceivedFromHero :type Boolean) (DamageType :type "/Game/RTS/Blueprints/Player/Data/Input/GestureDirection Enum" :default "NewEnumerator0") (DamageAmount :type Integer) (DamageForce :type "Vector Structure") (Attacker :type "Actor Object Reference"))
  (bind (_asaethelad_player_character_base _bsuccess) (cast `/Game/RTS/Blueprints/Player/AetheladPlayerCharacter/AetheladPlayerCharacterBase` Attacker :!pure true))
  (bind (_shoulddie _receiveddamage) (`self.ApplyDamageTyped` DamageType DamageAmount))
  (if _receiveddamage
    (`Character.LaunchCharacter` (cast `/Game/RTS/Blueprints/AI/UnitCharacterBase` (`self.K2_GetPawn`) :!pure true) (`KismetMathLibrary.TransformDirection` (`self.GetTransform` Attacker) DamageForce) false false)
    (`NiagaraFunctionLibrary.SpawnSystemAtLocation` "/Game/RTS/Assets/Particles/Damage/Particle_Blood_Emitter_System.Particle_Blood_Emitter_System" (`self.K2_GetActorLocation` (`self.K2_GetPawn`)))
    (if _shoulddie
      (`self.CharacterDie`))
    (elif _bsuccess
      (`/Game/RTS/Blueprints/Player/AetheladPlayerCharacter/AetheladPlayerCharacterBase.AttackStun` _asaethelad_player_character_base))))

(fn `ApplyDamageTyped`
  (params (DamageType :type "/Game/RTS/Blueprints/Player/Data/Input/GestureDirection Enum" :default "NewEnumerator0") (DamageAmount :type Integer))
  (returns (ShouldDie :type Boolean) (ReceivedDamage :type Boolean))
  (locals (StartingHealth :type Integer))
  (bind _health (`self.Health`))
  (bind (_maxhealth _maxmagic _maxstamina _piercethreshold _pierceresistance _slashthreshold _slashresistance _bludgeonthreshold _bludgeonresistance) (break `/Game/RTS/Blueprints/Player/Data/Character/CharacterStats` (`self.UnitStats`)))
  (set `local.StartingHealth` (`self.Health`))
  (switch `/Game/RTS/Blueprints/Player/Data/Input/GestureDirection` DamageType
    (:`NewEnumerator0`
      (set `self.Health` (- _health (`KismetMathLibrary.FTrunc` (* (- DamageAmount _slashthreshold) (- 1.0 _slashresistance)))) :!label _label))
    (:`NewEnumerator1`
      (goto _label))
    (:`NewEnumerator2`
      (set `self.Health` (- _health (`KismetMathLibrary.FTrunc` (* (- DamageAmount _piercethreshold) (- 1.0 _pierceresistance))))))
    (:`NewEnumerator3`
      (set `self.Health` (- _health (`KismetMathLibrary.FTrunc` (* (- DamageAmount _bludgeonthreshold) (- 1.0 _bludgeonresistance)))))))
  (return (<= (`self.Health`) 0) (< (`self.Health`) (`local.StartingHealth`))))

(fn `UserConstructionScript`)