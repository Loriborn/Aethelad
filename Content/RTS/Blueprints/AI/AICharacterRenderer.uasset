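; Actor that renders all RTS AI units as instances of a single Hierarchical Instanced Static Mesh.
; Shortly after BeginPlay it registers with the game instance, gathers every UnitCharacterBase, adds an instance for each and stores that index on its AI controller.
; Tick syncs instance transforms to units with mesh offsets, using a distance check meant to skip unmoved ones.
; RemoveUnit deletes the unit and instance, then decrements later controllers' indices.
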(event `RemoveUnit`
  (params (Index :type Integer))
  (`KismetArrayLibrary.Array_Remove` (`self.ArrayOfUnits`) Index)
  (`InstancedStaticMeshComponent.RemoveInstance` (`self.HierarchicalInstancedStaticMesh`) Index)
  (for _index (range Index (`KismetArrayLibrary.Array_Length` (`self.ArrayOfUnits`)))
    (bind _asunit_character_ai (cast `/Game/RTS/Blueprints/AI/UnitCharacterAI` (`Pawn.GetController` (`|GetArrayItem` (`self.ArrayOfUnits`) _index)) :!pure true))
    (set `/Game/RTS/Blueprints/AI/UnitCharacterAI.Index` (- (`/Game/RTS/Blueprints/AI/UnitCharacterAI.Index` _asunit_character_ai) 1) _asunit_character_ai)))

(event `self.ReceiveBeginPlay`
  (`KismetSystemLibrary.Delay` 0.2)
  (set `/Game/RTS/Blueprints/Game/AetheladGameInstance.AIUnitCharacterRenderer` self (cast `/Game/RTS/Blueprints/Game/AetheladGameInstance` (`GameplayStatics.GetGameInstance`) :!pure true))
  (bind _outactors (`GameplayStatics.GetAllActorsOfClass` "/Game/RTS/Blueprints/AI/UnitCharacterBase.UnitCharacterBase_C"))
  (bind _output_get (set `self.ArrayOfUnits` _outactors))
  (for (_array_element _array_index) _output_get
    (bind _asunit_character_ai (cast `/Game/RTS/Blueprints/AI/UnitCharacterAI` (`Pawn.GetController` _array_element) :!pure true))
    (set `/Game/RTS/Blueprints/AI/UnitCharacterAI.Index` _array_index _asunit_character_ai)
    (bind (_returnvalue_location _returnvalue_rotation) (`KismetMathLibrary.BreakTransform` (`self.GetTransform` _asunit_character_ai)))
    (`InstancedStaticMeshComponent.AddInstanceWorldSpace` (`self.HierarchicalInstancedStaticMesh`) (`KismetMathLibrary.MakeTransform` _returnvalue_location _returnvalue_rotation (5.0 5.0 5.0)))))

(event `self.ReceiveTick`
  (params (DeltaSeconds :type "Float (single-precision)"))
  (bind _arrayofunits (`self.ArrayOfUnits`))
  (bind _hierarchicalinstancedstaticmesh (`self.HierarchicalInstancedStaticMesh`))
  (if (> (`KismetArrayLibrary.Array_Length` _arrayofunits) 0)
    (for (_array_element _array_index) _arrayofunits
      (`/Engine/EditorBlueprintResources/StandardMacros.IsValid` _array_element
        (:`Is Valid`
          (bind (_returnvalue_location _returnvalue_rotation) (`KismetMathLibrary.BreakTransform` (`self.GetTransform` _array_element)))
          (if (not (== _returnvalue_location (.location (`InstancedStaticMeshComponent.GetInstanceTransform` _hierarchicalinstancedstaticmesh _array_index true)) :`ErrorTolerance` 2.0))
            (`InstancedStaticMeshComponent.UpdateInstanceTransform` _hierarchicalinstancedstaticmesh _array_index (`KismetMathLibrary.MakeTransform` (`KismetMathLibrary.MakeVector` (.x _returnvalue_location) (.y _returnvalue_location) (- (.z _returnvalue_location) 90.0)) (`KismetMathLibrary.ComposeRotators` _returnvalue_rotation (struct :`Yaw` -90.0)) (5.0 5.0 5.0)) true false false)))))))

(fn `UserConstructionScript`)