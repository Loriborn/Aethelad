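; Base item Blueprint for the RTS game, handling equip physics and modifiable value and weight stats.
; Equipping turns off mesh physics and collision; unequipping restores both.
; CompressTagData writes the modified totals into a string TagData map.
; DecompressTagData parses that map, adding each entry to BaseValue, even for weight, so stored totals are treated as offsets.
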(event `OnItemUnequip`
  (bind _itemmesh (`self.ItemMesh`))
  (`PrimitiveComponent.SetCollisionEnabled` _itemmesh "QueryAndPhysics")
  (`PrimitiveComponent.SetSimulatePhysics` _itemmesh true))

(event `OnItemEquip`
  (bind _itemmesh (`self.ItemMesh`))
  (`PrimitiveComponent.SetSimulatePhysics` _itemmesh false)
  (`PrimitiveComponent.SetCollisionEnabled` _itemmesh "NoCollision"))

(event `DecompressTagData`
  (params (TagData :type "Map of Name to String"))
  (bind _output_get (set `self.TagData` TagData))
  (bind _keys (`BlueprintMapLibrary.Map_Keys` _output_get))
  (for _array_element _keys
    (switch `name` _array_element
      (:`VALUE_MODIFIER`
        (bind _returnvalue (`KismetStringLibrary.Conv_StringToDouble` (`BlueprintMapLibrary.Map_Find` _output_get _array_element)))
        (set `self.ModifiedValue` (+ (`self.BaseValue`) _returnvalue)))
      (:`WEIGHT_MODIFIER`
        (set `self.ModifiedWeight` (+ (`self.BaseValue`) _returnvalue))))))

(event `CompressTagData`
  (bind _tagdata (`self.TagData`))
  (`BlueprintMapLibrary.Map_Clear` _tagdata)
  (`BlueprintMapLibrary.Map_Add` _tagdata "VALUE_MODIFIER" (`KismetStringLibrary.Conv_DoubleToString` (`self.ModifiedValue`)))
  (`BlueprintMapLibrary.Map_Add` _tagdata "WEIGHT_MODIFIER" (`KismetStringLibrary.Conv_DoubleToString` (`self.ModifiedWeight`))))

(fn `UserConstructionScript`)