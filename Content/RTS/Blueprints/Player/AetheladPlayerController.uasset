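; Player controller that routes UI input actions to container popups, for browsing and transferring items between the player and an interacted entity.
; CheckValidPopup fetches the character's active popup, which the move inputs navigate by row or column as a UI_Container.
; Cycle inputs step the clamped ActivePopup index and shift container focus.
; Accept places or takes the selected item on the Entity_Container, depending on whether the popup is linked to the player.
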(event `InputAction|UIMoveLeft` :consume false
  (params (Key :type "Key Structure"))
  (:`Pressed`
    (bind (_isvalid _widgetreference) (`self.CheckValidPopup`))
    (if _isvalid
      (bind _asui_container (cast `/Game/RTS/Blueprints/UI/Widgets/Containers/UI_Container` _widgetreference))
      (`/Game/RTS/Blueprints/UI/Widgets/Containers/UI_Container.MoveColumn` _asui_container false))))

(event `InputAction|UIMoveRight` :consume false
  (params (Key :type "Key Structure"))
  (:`Pressed`
    (bind (_isvalid _widgetreference) (`self.CheckValidPopup`))
    (if _isvalid
      (bind _asui_container (cast `/Game/RTS/Blueprints/UI/Widgets/Containers/UI_Container` _widgetreference))
      (`/Game/RTS/Blueprints/UI/Widgets/Containers/UI_Container.MoveColumn` _asui_container true))))

(event `InputAction|UIMoveUp` :consume false
  (params (Key :type "Key Structure"))
  (:`Pressed`
    (bind (_isvalid _widgetreference) (`self.CheckValidPopup`))
    (if _isvalid
      (bind _asui_container (cast `/Game/RTS/Blueprints/UI/Widgets/Containers/UI_Container` _widgetreference))
      (`/Game/RTS/Blueprints/UI/Widgets/Containers/UI_Container.MoveRow` _asui_container true))))

(event `InputAction|UIMoveDown` :consume false
  (params (Key :type "Key Structure"))
  (:`Pressed`
    (bind (_isvalid _widgetreference) (`self.CheckValidPopup`))
    (if _isvalid
      (bind _asui_container (cast `/Game/RTS/Blueprints/UI/Widgets/Containers/UI_Container` _widgetreference))
      (`/Game/RTS/Blueprints/UI/Widgets/Containers/UI_Container.MoveRow` _asui_container false))))

(event `InputAction|UICycleBack` :consume false
  (params (Key :type "Key Structure"))
  (bind _asaethelad_player_character_base (cast `/Game/RTS/Blueprints/Player/AetheladPlayerCharacter/AetheladPlayerCharacterBase` (`self.K2_GetPawn`) :!pure true))
  (bind _output (`|GetArrayItem` (`/Game/RTS/Blueprints/Player/AetheladPlayerCharacter/AetheladPlayerCharacterBase.PopupReferences` _asaethelad_player_character_base) (`/Game/RTS/Blueprints/Player/AetheladPlayerCharacter/AetheladPlayerCharacterBase.ActivePopup` _asaethelad_player_character_base)))
  (bind _returnvalue (`KismetMathLibrary.Clamp` (+ (`/Game/RTS/Blueprints/Player/AetheladPlayerCharacter/AetheladPlayerCharacterBase.ActivePopup` _asaethelad_player_character_base) 1) 0 (- (`KismetArrayLibrary.Array_Length` (`/Game/RTS/Blueprints/Player/AetheladPlayerCharacter/AetheladPlayerCharacterBase.PopupReferences` _asaethelad_player_character_base)) 1)))
  (:`Pressed`
    (if (not (== _returnvalue (`/Game/RTS/Blueprints/Player/AetheladPlayerCharacter/AetheladPlayerCharacterBase.ActivePopup` _asaethelad_player_character_base)))
      (bind _asui_container (cast `/Game/RTS/Blueprints/UI/Widgets/Containers/UI_Container` _output))
      (`/Game/RTS/Blueprints/UI/Widgets/Containers/UI_Container.RefocusContainer` _asui_container false)
      (set `/Game/RTS/Blueprints/Player/AetheladPlayerCharacter/AetheladPlayerCharacterBase.ActivePopup` _returnvalue _asaethelad_player_character_base)
      (`/Game/RTS/Blueprints/UI/Widgets/Containers/UI_Container.RefocusContainer` (cast `/Game/RTS/Blueprints/UI/Widgets/Containers/UI_Container` _output :!pure true) true))))

(event `InputAction|UICycleForward` :consume false
  (params (Key :type "Key Structure"))
  (bind _asaethelad_player_character_base (cast `/Game/RTS/Blueprints/Player/AetheladPlayerCharacter/AetheladPlayerCharacterBase` (`self.K2_GetPawn`) :!pure true))
  (bind _output (`|GetArrayItem` (`/Game/RTS/Blueprints/Player/AetheladPlayerCharacter/AetheladPlayerCharacterBase.PopupReferences` _asaethelad_player_character_base) (`/Game/RTS/Blueprints/Player/AetheladPlayerCharacter/AetheladPlayerCharacterBase.ActivePopup` _asaethelad_player_character_base)))
  (bind _returnvalue (`KismetMathLibrary.Clamp` (- (`/Game/RTS/Blueprints/Player/AetheladPlayerCharacter/AetheladPlayerCharacterBase.ActivePopup` _asaethelad_player_character_base) 1) 0 (- (`KismetArrayLibrary.Array_Length` (`/Game/RTS/Blueprints/Player/AetheladPlayerCharacter/AetheladPlayerCharacterBase.PopupReferences` _asaethelad_player_character_base)) 1)))
  (:`Pressed`
    (if (not (== (`/Game/RTS/Blueprints/Player/AetheladPlayerCharacter/AetheladPlayerCharacterBase.ActivePopup` _asaethelad_player_character_base) _returnvalue))
      (bind _asui_container (cast `/Game/RTS/Blueprints/UI/Widgets/Containers/UI_Container` _output))
      (`/Game/RTS/Blueprints/UI/Widgets/Containers/UI_Container.RefocusContainer` _asui_container false)
      (set `/Game/RTS/Blueprints/Player/AetheladPlayerCharacter/AetheladPlayerCharacterBase.ActivePopup` _returnvalue _asaethelad_player_character_base)
      (`/Game/RTS/Blueprints/UI/Widgets/Containers/UI_Container.RefocusContainer` (cast `/Game/RTS/Blueprints/UI/Widgets/Containers/UI_Container` _output :!pure true) true))))

(event `InputAction|UIDecline`
  (params (Key :type "Key Structure")))

(event `InputAction|UIAccept` :consume false
  (params (Key :type "Key Structure"))
  (:`Pressed`
    (bind (_isvalid _widgetreference _user) (`self.CheckValidPopup`))
    (if _isvalid
      (bind _asui_container (cast `/Game/RTS/Blueprints/UI/Widgets/Containers/UI_Container` _widgetreference))
      (bind _asentity_container (cast `/Game/RTS/Blueprints/World/Entities/Entity_Container` (`/Game/RTS/Blueprints/Player/AetheladPlayerCharacter/AetheladPlayerCharacterBase.InteractingEntity` _user)))
      (if (== (`/Game/RTS/Blueprints/UI/Widgets/Containers/UI_Container.LinkedActor` _asui_container) _user)
        (bind _playeractiveitemindex (`/Game/RTS/Blueprints/UI/Widgets/Containers/UI_Container.PlayerActiveItemIndex` _asui_container))
        (`/Game/RTS/Blueprints/World/Entities/Entity_Container.AttemptPlaceItem` _asentity_container _user _playeractiveitemindex)
        (else
          (`/Game/RTS/Blueprints/World/Entities/Entity_Container.AttemptTakeItem` _asentity_container _user _playeractiveitemindex))))))

(fn `CheckValidPopup`
  (returns (IsValid :type Boolean) (WidgetReference :type "UserWidget Object Reference") (User :type "/Game/RTS/Blueprints/Player/AetheladPlayerCharacter/AetheladPlayerCharacterBase Object Reference"))
  (bind _asaethelad_player_character_base (cast `/Game/RTS/Blueprints/Player/AetheladPlayerCharacter/AetheladPlayerCharacterBase` (`self.K2_GetPawn`) :!pure true))
  (bind _output (`|GetArrayItem` (`/Game/RTS/Blueprints/Player/AetheladPlayerCharacter/AetheladPlayerCharacterBase.PopupReferences` _asaethelad_player_character_base) (`/Game/RTS/Blueprints/Player/AetheladPlayerCharacter/AetheladPlayerCharacterBase.ActivePopup` _asaethelad_player_character_base)))
  (`/Engine/EditorBlueprintResources/StandardMacros.IsValid` _output
    (:`Is Valid`
      (return true _output _asaethelad_player_character_base))
    (:`Is Not Valid`
      (return false null _asaethelad_player_character_base))))

(fn `UserConstructionScript`)